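; BP_Yoshi is a character Blueprint in the players folder that handles death by shock and being stomped on the head.
; Overlapping a BP_Shock actor disables player input, launches the character along negative X and upward, and clears IsAlive.
; When another UE_TakeMeOhmCharacter overlaps HeadCollider, that character gets an upward velocity-change impulse, while Yoshi sets Stomped and deactivates the collider.
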(event `self.ReceiveActorBeginOverlap`
  (params (OtherActor :type "Actor Object Reference"))
  (cast `/Game/BP_Shock` OtherActor)
  (bind _asplayer_controller (cast `PlayerController` (`self.GetController`)))
  (`self.DisableInput` _asplayer_controller)
  (`self.LaunchCharacter` (-1000.0 0.0 1000.0))
  (set `self.IsAlive` false))

(event `self.HeadCollider.OnComponentBeginOverlap`
  (params (OverlappedComponent :type "PrimitiveComponent Object Reference") (OtherActor :type "Actor Object Reference") (OtherComp :type "PrimitiveComponent Object Reference") (OtherBodyIndex :type Integer) (bFromSweep :type Boolean) (SweepResult :type "HitResult Structure (by ref)"))
  (if (!= OtherActor self)
    (bind _asue_take_me_ohm_character (cast `UE_TakeMeOhmCharacter` OtherActor))
    (`CharacterMovementComponent.AddImpulse` (`Character.CharacterMovement` _asue_take_me_ohm_character) (0.0 0.0 1000.0) true)
    (`self.SetStomped` true)
    (`ActorComponent.Deactivate` (`self.HeadCollider`))))

(fn `UserConstructionScript`)