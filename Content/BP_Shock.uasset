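; BP_Shock is a shockwave actor that slides along its local X axis each tick, widens, then destroys itself.
; A timeline, played from Tick, drives the box collision extent and sets the particle beam's endpoints from its Y scale.
; The beam endpoints are offset along world X, ignoring actor rotation, and movement is per frame without sweep or delta-time scaling.
; The graph contains no hit or damage logic.
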(event `self.ReceiveTick`
  (params (DeltaSeconds :type "Float (single-precision)"))
  (bind (_returnvalue_x _returnvalue_y _returnvalue_z) (`KismetMathLibrary.BreakVector` (`self.K2_GetActorLocation`)))
  (bind _particlesystem (`self.ParticleSystem`))
  (`self.K2_AddActorLocalOffset` (7.5 0.0 0.0))
  (bind (_direction _scale) (`Timeline|ScaleTimeLine`)
    (:`Update`
      (`BoxComponent.SetBoxExtent` (`self.Box`) (`KismetMathLibrary.MakeVector` (.x _scale) (.y _scale) (.z _scale)) true)
      (bind _result (`/Engine/EditorBlueprintResources/StandardMacros.NegateFloat` (.y _scale))
        (:`  `
          (`ParticleSystemComponent.SetBeamSourcePoint` _particlesystem 0 (`KismetMathLibrary.MakeVector` (+ _result _returnvalue_x) _returnvalue_y _returnvalue_z) 0)
          (`ParticleSystemComponent.SetBeamEndPoint` _particlesystem 0 (`KismetMathLibrary.MakeVector` (+ (.y _scale) _returnvalue_x) _returnvalue_y _returnvalue_z)))))
    (:`Finished`
      (`self.K2_DestroyActor`))))

(fn `UserConstructionScript`)