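; BP_Thwomp is a Thwomp-style block that drops under physics and climbs back up.
; Fall enables physics on the Box and clears Idle; any actor overlap sets OnGround, which is never cleared here.
; While OnGround, Tick counts to IdleTime, then disables physics and starts rising.
; The rise uses a fixed, unswept per-frame offset until UpTime elapses, then sets Idle.
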(event `self.ReceiveActorBeginOverlap`
  (params (OtherActor :type "Actor Object Reference"))
  (set `self.OnGround` true))

(event `self.ReceiveTick`
  (params (DeltaSeconds :type "Float (single-precision)"))
  (`|ExecutionSequence`
    (:`then_0`
      (if (`self.OnGround`)
        (bind _output_get (set `self.ActualTime` (+ DeltaSeconds (`self.ActualTime`))))
        (if (>= _output_get (`self.IdleTime`))
          (set `self.GettingUp` true)
          (set `self.ActualTime` 0.0)
          (`PrimitiveComponent.SetSimulatePhysics` (`self.Box`) false))))
    (:`then_1`
      (if (`self.GettingUp`)
        (bind _output_get_2 (set `self.ActualUpTime` (+ DeltaSeconds (`self.ActualUpTime`))))
        (if (>= _output_get_2 (`self.UpTime`))
          (set `self.ActualUpTime` 0.0)
          (set `self.GettingUp` false)
          (set `self.Idle` true)
          (else
            (`self.K2_AddActorLocalOffset` (0.0 0.0 5.0))))))))

(fn `Fall`
  (`PrimitiveComponent.SetSimulatePhysics` (`self.Box`) true)
  (set `self.Idle` false))

(fn `UserConstructionScript`)